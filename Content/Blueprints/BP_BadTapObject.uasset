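; BP_BadTapObject is the bad variant of a tappable sprite object in a touch-based scoring game.
; On BeginPlay it sets IsGoodTapObject to false, then runs the parent's BeginPlay logic.
; Touching its PaperSprite calls EventOnTapBadObject on the game mode reference and destroys the actor, leaving the penalty to the game mode.
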(event OnInputTouchBegin(PaperSprite)
  (params (FingerIndex :type ETouchIndex%20Enum :default "Touch1") (TouchedComponent :type Primitive%20Component%20Object%20Reference))
  (Default|EventonTapBadObject (Variables|Default|GetAs%20BP%20Game%20Mode))
  (Development|PrintString "Reduce Score!" false false)
  (Actor|DestroyActor))

(event EventBeginPlay
  (Variables|Default|SetisGoodTapObject false)
  (|CallParentFunction))

(event Collision|EventActorBeginOverlap
  (params (OtherActor :type Actor%20Object%20Reference))
  (|CallParentFunction OtherActor) ; This node is disabled and will not be called.\nDrag off pins to build functionality.
)

(event EventTick
  (params (DeltaSeconds :type Float%20%28single-precision%29))
  (|CallParentFunction DeltaSeconds) ; This node is disabled and will not be called.\nDrag off pins to build functionality.
)

(fn ConstructionScript
  (|CallParentFunction))