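; BP_TapObject is a tappable sprite actor that appears as a bomb, good or bad object and expires after a short time.
; On BeginPlay it picks a sprite from its type flags, randomizes its pitch, then animates rotation with a timeline.
; Timeline updates also cache BP_GameMode and start a delay, using its destroy interval, before destruction.
; Touch calls the GameMode's good-object tap event for every type, then destroys the actor.
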(event OnInputTouchBegin(PaperSprite)
  (params (FingerIndex :type ETouchIndex%20Enum :default "Touch1") (TouchedComponent :type Primitive%20Component%20Object%20Reference))
  (Default|EventonTapGoodObject (Variables|Default|GetAs%20BP%20Game%20Mode))
  (Development|PrintString "Increase Score!" false false)
  (Actor|DestroyActor))

(event EventBeginPlay
  (Utilities|SelectArrayOfSprite
    (:output
      (Utilities|InitRotationShape)
      (bind _rotate_right (Timeline|RotateTimeline Play)
        (:Update
          (Transformation|SetActorRotation (Math|Rotator|MakeRotator 0.0 _rotate_right 0.0))
          (bind _asbp_game_mode (Utilities|Casting|CastToBP_GameMode (Game|GetGameMode)))
          (Development|PrintString "GameMode Set!" false false)
          (bind _output_get (Variables|Default|SetAs%20BP%20Game%20Mode _asbp_game_mode))
          (Utilities|FlowControl|Delay (Variables|/Game/Blueprints/BP_GameMode.BP_GameMode_C|GetdestroyTapObjectInterval _output_get))
          (Actor|DestroyActor))))))

(event Collision|EventActorBeginOverlap
  (params (OtherActor :type Actor%20Object%20Reference)))

(event EventTick
  (params (DeltaSeconds :type Float%20%28single-precision%29)))

(fn ConstructionScript)