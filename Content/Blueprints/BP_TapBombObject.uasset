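; BP_TapBombObject is the bomb variant of a tappable object, ending the game when the player touches it.
; On BeginPlay it flags itself as a bomb rather than a good object, then runs the parent's setup.
; A touch on its PaperSprite sets GameOver on the game mode, disables input, and shows a BP_GameOverHUD widget with the final score.
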(event OnInputTouchBegin(PaperSprite)
  (params (FingerIndex :type ETouchIndex%20Enum :default "Touch1") (TouchedComponent :type Primitive%20Component%20Object%20Reference))
  (Variables|/Game/Blueprints/BP_GameMode.BP_GameMode_C|SetGameOver (Variables|Default|GetAs%20BP%20Game%20Mode) true)
  (Input|DisableInput (Game|GetPlayerController 0))
  (bind _returnvalue (UserInterface|CreateWidget "/Game/Blueprints/BP_GameOverHUD.BP_GameOverHUD_C" (Game|GetPlayerController 0)))
  (Default|ChangeFinalScore _returnvalue (Variables|/Game/Blueprints/BP_GameMode.BP_GameMode_C|GetScore (Variables|Default|GetAs%20BP%20Game%20Mode)))
  (UserInterface|Viewport|AddtoViewport _returnvalue 0))

(event EventBeginPlay
  (Variables|Default|SetisBombTapObject true)
  (Variables|Default|SetisGoodTapObject false)
  (|CallParentFunction))

(fn ConstructionScript
  (|CallParentFunction))