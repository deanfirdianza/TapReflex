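; Game mode for a tapping game that creates the HUD, tracks score and handles game over.
; Good taps raise score and tap count, bad taps lower score, and both update the HUD and run the difficulty check.
; That check shortens clamped spawn and destroy intervals at set tap-count multiples, then adds bad and bomb classes at a fixed count.
; A bomb tap removes the HUD and sets GameOver, prompting Tick to destroy the spawner.
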(event Custom|Event%20OnTapGoodObject
  (bind _tappableclass (Variables|Default|GetTappableClass))
  (Variables|Default|SetTapCounter (+ (Variables|Default|GetTapCounter) 1))
  (Development|PrintString "Good Object" false false)
  (bind _output_get (Variables|Default|SetScore (+ (Variables|Default|GetScore) 1)))
  (Development|PrintString "GoodTap")
  (Default|UpdateScore (Variables|Default|GetAs%20BP%20HUD) (Utilities|Text|ToText(Integer) _output_get))
  (Utilities|IsTapReduceInterval
    (:output
      (if (== (Variables|Default|GetTapCounter) 6)
        (Utilities|Array|Add _tappableclass "/Game/Blueprints/BP_BadTapObject.BP_BadTapObject_C")
        (Utilities|Array|Add _tappableclass "/Game/Blueprints/BP_TapBombObject.BP_TapBombObject_C")
        (for _array_element _tappableclass
          (Development|PrintString (Utilities|GetClassDisplayName _array_element) false false))))))

(event Custom|Event%20OnTapBadObject
  (bind _tappableclass (Variables|Default|GetTappableClass))
  (bind _output_get (Variables|Default|SetScore (- (Variables|Default|GetScore) 1)))
  (Development|PrintString "BadTap")
  (Default|UpdateScore (Variables|Default|GetAs%20BP%20HUD) (Utilities|Text|ToText(Integer) _output_get))
  (Utilities|IsTapReduceInterval
    (:output
      (if (== (Variables|Default|GetTapCounter) 6)
        (Utilities|Array|Add _tappableclass "/Game/Blueprints/BP_BadTapObject.BP_BadTapObject_C")
        (Utilities|Array|Add _tappableclass "/Game/Blueprints/BP_TapBombObject.BP_TapBombObject_C")
        (for _array_element _tappableclass
          (Development|PrintString (Utilities|GetClassDisplayName _array_element) false false))))))

(event Custom|Event%20OnTapBombObject
  (Variables|Default|SetGameOver true)
  (Widget|RemovefromParent (Variables|Default|GetAs%20BP%20HUD)))

(event EventBeginPlay
  (bind _returnvalue (UserInterface|CreateWidget "/Game/Blueprints/BP_HUD.BP_HUD_C" (Game|GetPlayerController 0)))
  (UserInterface|Viewport|AddtoViewport _returnvalue 0)
  (Variables|Default|SetAs%20BP%20HUD _returnvalue))

(event EventTick
  (params (DeltaSeconds :type Float%20%28single-precision%29))
  (if (Variables|Default|GetGameOver)
    (if (Utilities|IsValid (Variables|Default|GetAs%20BP%20Spawner))
      (Actor|DestroyActor (Variables|Default|GetAs%20BP%20Spawner))
      (Variables|Default|SetAs%20BP%20Spawner 0))))

(fn ConstructionScript)